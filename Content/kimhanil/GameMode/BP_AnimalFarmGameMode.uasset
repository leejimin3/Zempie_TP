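; Game mode for an animal farm game that populates the level with ten animals when play begins.
; BeginPlay and a custom Spawn event share one call to SpawnAnimals, which is not defined in this graph.
; An unconnected test chain breeds a child from the first two animals with MakeChildAnimal and prints its Head, Body, Tail and Leg arrays.
; Tick and the construction script are empty.
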(event Custom|Spawn
  (Class|AnimalFarmGameMode|SpawnAnimals 10))

(event EventBeginPlay
  (Class|AnimalFarmGameMode|SpawnAnimals 10))

(event EventTick
  (params (DeltaSeconds :type Float%20%28single-precision%29)))

(fn ConstructionScript)