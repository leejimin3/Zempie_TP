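; Blueprint that assembles a composite animal picture from head, body, leg and tail Paper2D sprites.
; Init looks up each of the animal's codes in BP_AnimalFarmGameMode's image data, assigning sprites and collecting pin points and sizes.
; It then positions head, leg and tail relative to the body by aligning pins, converting pixel coordinates to centred offsets.
; Sprites and texture sizes are found through Asset Registry folder scans matched by name substring.
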(event Custom|Init
  (params (Animal :type Parent%20Animal%20Object%20Reference) (Head :type Paper%20Sprite%20Component%20Object%20Reference) (Body :type Paper%20Sprite%20Component%20Object%20Reference) (Leg :type Paper%20Sprite%20Component%20Object%20Reference) (Tail :type Paper%20Sprite%20Component%20Object%20Reference) (타깃 :type Self%20Object%20Reference))
  (Utilities|FlowControl|Sequence
    (:then_0
      (Variables|Default|SetAnimalPartsSprites (Utilities|Array|MakeArray Head Leg Tail))
      (Variables|Default|SetAnimalBodySprite Body)
      (bind _asbp_animal_farm_game_mode (Utilities|Casting|CastToBP_AnimalFarmGameMode (Game|GetGameMode)))
      (for (_array_element _array_index) (Variables|/Script/TwoSomePlace.Parent_Animal|GetanimalCodes Animal)
        (bind _returnvalue (Class|AnimalFarmGameMode|GetAnimalImageData _asbp_animal_farm_game_mode _array_element))
        (switch int _array_index
          (:0
            (Utilities|Array|Add (Variables|Default|GetVectorBias) (.Value (Utilities|Map|Find (.imagevector2ddatas _returnvalue) "Head")))
            (bind _as페이퍼_스프라이트 (CallFunction|GetImage (.Value (Utilities|Map|Find (.texturenames _returnvalue) "Head"))))
            (Rendering|Components|Sprite|SetSprite Head _as페이퍼_스프라이트)
            (bind _imagesize (CallFunction|GetImageSize (.Value (Utilities|Map|Find (.texturenames _returnvalue) "Head"))))
            (Utilities|Array|Add (Variables|Default|GetImageSizes) _imagesize))
          (:1
            (Variables|Default|SetAnimalBodyPins (.Value (Utilities|Map|Find (.imagevector2ddatas _returnvalue) "Body")))
            (bind _as페이퍼_스프라이트_2 (CallFunction|GetImage (.Value (Utilities|Map|Find (.texturenames _returnvalue) "Body"))))
            (Rendering|Components|Sprite|SetSprite Body _as페이퍼_스프라이트_2)
            (bind _imagesize_2 (CallFunction|GetImageSize (.Value (Utilities|Map|Find (.texturenames _returnvalue) "Body"))))
            (Variables|Default|SetBodySize _imagesize_2))
          (:2
            (Utilities|Array|Add (Variables|Default|GetVectorBias) (.Value (Utilities|Map|Find (.imagevector2ddatas _returnvalue) "Leg")))
            (bind _as페이퍼_스프라이트_3 (CallFunction|GetImage (.Value (Utilities|Map|Find (.texturenames _returnvalue) "Leg"))))
            (Rendering|Components|Sprite|SetSprite Leg _as페이퍼_스프라이트_3)
            (bind _imagesize_3 (CallFunction|GetImageSize (.Value (Utilities|Map|Find (.texturenames _returnvalue) "Leg"))))
            (Utilities|Array|Add (Variables|Default|GetImageSizes) _imagesize_3))
          (:3
            (Utilities|Array|Add (Variables|Default|GetVectorBias) (.Value (Utilities|Map|Find (.imagevector2ddatas _returnvalue) "Tail")))
            (bind _as페이퍼_스프라이트_4 (CallFunction|GetImage (.Value (Utilities|Map|Find (.texturenames _returnvalue) "Tail"))))
            (Rendering|Components|Sprite|SetSprite Tail _as페이퍼_스프라이트_4)
            (bind _imagesize_4 (CallFunction|GetImageSize (.Value (Utilities|Map|Find (.texturenames _returnvalue) "Tail"))))
            (Utilities|Array|Add (Variables|Default|GetImageSizes) _imagesize_4)))))
    (:then_1
      (for (_array_element_2 _array_index_2) (Variables|Default|GetAnimalPartsSprites)
        (Utilities|IsValid _array_element_2
          (:Is%20Valid
            (Transformation|SetRelativeLocation _array_element_2 (Math|Vector|MakeVector (+ (+ (.x (Utilities|Array|Get(acopy) (Utilities|Struct|BreakVector2Ds (Variables|Default|GetAnimalBodyPins)) (+ _array_index_2 1))) (/ (.x (Variables|Default|GetBodySize)) -2.0)) (+ (.x (Utilities|Array|Get(acopy) (.vector2ds (Utilities|Array|Get(acopy) (Variables|Default|GetVectorBias) _array_index_2)))) (/ (.x (Utilities|Array|Get(acopy) (Variables|Default|GetImageSizes) _array_index_2)) 2.0))) 0.0 (+ (- (/ (.y (Variables|Default|GetBodySize)) 2.0) (.y (Utilities|Array|Get(acopy) (Utilities|Struct|BreakVector2Ds (Variables|Default|GetAnimalBodyPins)) (+ _array_index_2 1)))) (- (.y (Utilities|Array|Get(acopy) (.vector2ds (Utilities|Array|Get(acopy) (Variables|Default|GetVectorBias) _array_index_2)))) (/ (.y (Utilities|Array|Get(acopy) (Variables|Default|GetImageSizes) _array_index_2)) 2.0)))) false false)))))))

(event EventBeginPlay)

(fn GetImage
  (params (ImageName :type String))
  (bind _outassetdata (Class|AssetRegistry|GetAssetsbyPath (Class|AssetRegistryHelpers|GetAssetRegistry) "/Game/AnimalImages" false false))
  (for _array_element _outassetdata
    (if (Utilities|String|Contains (Class|AssetRegistryHelpers|GetFullName _array_element) ImageName)
      (bind _as페이퍼_스프라이트 (Utilities|Casting|CastToPaperSprite (Class|AssetRegistryHelpers|GetAsset _array_element)))
      (return _as페이퍼_스프라이트))))

(fn GetImageSize
  (params (InputPin :type String))
  (bind _outassetdata (Class|AssetRegistry|GetAssetsbyPath (Class|AssetRegistryHelpers|GetAssetRegistry) "/Game/AnimalImages/RawImages" false false))
  (for _array_element _outassetdata
    (if (Utilities|String|Contains (Class|AssetRegistryHelpers|GetFullName _array_element) InputPin)
      (bind _as텍스처_2d (Utilities|Casting|CastToTexture2D (Class|AssetRegistryHelpers|GetAsset _array_element)))
      (return (Math|Vector2D|MakeVector2D (Math|Conversions|ToFloat(Integer) (Class|Texture2D|BlueprintGetSizeX _as텍스처_2d)) (Math|Conversions|ToFloat(Integer) (Class|Texture2D|BlueprintGetSizeY _as텍스처_2d)))))))